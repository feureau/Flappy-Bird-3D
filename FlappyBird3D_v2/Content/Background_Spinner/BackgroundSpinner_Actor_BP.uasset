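; BackgroundSpinner_Actor_BP is the Flappy Bird-style background spinner actor that hosts the pipe obstacles and the lethal ceiling and floor.
; On BeginPlay it passes its pipe count to SpawnObstacles on an Obstacle_Spawner_BP held in a child actor component.
; Hits on either death collider call KillBird on the bird character, tagged with the collider's name.
; An older, unconnected chain for offsetting and configuring the spawner never runs.
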(event `self.ReceiveBeginPlay`
  (bind _asobstacle_spawner_bp (cast `/Game/Background_Spinner/Obstacle_Spawner_BP` (`ChildActorComponent.ChildActor` (`self.Obstacle_Spawner_BP`))))
  (`/Game/Background_Spinner/Obstacle_Spawner_BP.Spawn Obstacles` _asobstacle_spawner_bp (`self.Total number of pipes`)))

(event `self.DeathCollider_Ceiling.OnComponentHit`
  (params (HitComponent :type "PrimitiveComponent Object Reference") (OtherActor :type "Actor Object Reference") (OtherComp :type "PrimitiveComponent Object Reference") (NormalImpulse :type "Vector Structure") (Hit :type "HitResult Structure (by ref)"))
  (bind _asflappy_bird_character_bp (cast `/Game/FlappyBird/FlappyBird_Character_BP` OtherActor))
  (`/Game/FlappyBird/FlappyBird_Character_BP.Kill Bird` _asflappy_bird_character_bp "DeathCollider_Ceiling"))

(event `self.DeathCollider_Floor.OnComponentHit`
  (params (HitComponent :type "PrimitiveComponent Object Reference") (OtherActor :type "Actor Object Reference") (OtherComp :type "PrimitiveComponent Object Reference") (NormalImpulse :type "Vector Structure") (Hit :type "HitResult Structure (by ref)"))
  (bind _asflappy_bird_character_bp (cast `/Game/FlappyBird/FlappyBird_Character_BP` OtherActor))
  (`/Game/FlappyBird/FlappyBird_Character_BP.Kill Bird` _asflappy_bird_character_bp "DeathCollider_Floor"))

(fn `UserConstructionScript`)