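; Spawner Blueprint that places a requested number of Obstacles_BP pipe obstacles evenly around a circular spline path.
; The SpawnObstacles event finds the CircularSpline_BP by "Pipe Path" tag and spawns at world-space transforms spaced by spline length over count.
; The SpawnPipes function repeats this with a class lookup and local-space transforms.
; Indexing starts at 1 to avoid overlapping obstacles where the loop closes.
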(event `Spawn Obstacles`
  (params (`Number of Obstacles to spawn` :type Integer))
  (set `self.Total Number of Pipes` `Number of Obstacles to spawn`)
  (bind _outactors (`GameplayStatics.GetAllActorsWithTag` "Pipe Path"))
  (bind _ascircular_spline_bp (cast `/Game/Background_Spinner/CircularSpline_BP` (`|GetArrayItem` _outactors)))
  (set `self.Circular Spline That is the Main Path` _ascircular_spline_bp)
  (for _index (range 1 (+ (`self.Total Number of Pipes`) 1))
    (`|SpawnActorFromClass` "/Game/Obstacles/Obstacles_BP.Obstacles_BP_C" (`SplineComponent.GetTransformAtDistanceAlongSpline` (`/Game/Background_Spinner/CircularSpline_BP.Circle_Spline` (`self.Circular Spline That is the Main Path`)) (* _index (/ (`SplineComponent.GetSplineLength` (`/Game/Background_Spinner/CircularSpline_BP.Circle_Spline` (`self.Circular Spline That is the Main Path`))) (`KismetMathLibrary.Conv_IntToDouble` (`self.Total Number of Pipes`)))) "World" false) "AlwaysSpawn" "OverrideRootScale" null null)))

(fn `Spawn pipes`
  (params (`Number of pipes to spawn` :type Integer))
  (set `self.Total Number of Pipes` `Number of pipes to spawn`)
  (bind _outactors (`GameplayStatics.GetAllActorsOfClass` "/Game/Background_Spinner/CircularSpline_BP.CircularSpline_BP_C"))
  (bind _ascircular_spline_bp (cast `/Game/Background_Spinner/CircularSpline_BP` (`|GetArrayItem` _outactors)))
  (set `self.Circular Spline That is the Main Path` _ascircular_spline_bp)
  (for _index (range 1 (+ (`self.Total Number of Pipes`) 1))
    (`|SpawnActorFromClass` "/Game/Obstacles/Obstacles_BP.Obstacles_BP_C" (`SplineComponent.GetTransformAtDistanceAlongSpline` (`/Game/Background_Spinner/CircularSpline_BP.Circle_Spline` (`self.Circular Spline That is the Main Path`)) (* _index (/ (`SplineComponent.GetSplineLength` (`/Game/Background_Spinner/CircularSpline_BP.Circle_Spline` (`self.Circular Spline That is the Main Path`))) (`KismetMathLibrary.Conv_IntToDouble` (`self.Total Number of Pipes`)))) "Local" false) "AlwaysSpawn" "OverrideRootScale" null null)))

(fn `UserConstructionScript`)