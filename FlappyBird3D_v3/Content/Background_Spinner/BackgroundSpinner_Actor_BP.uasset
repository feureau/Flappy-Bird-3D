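; Background spinner actor for a Flappy Bird-style game that lays out the pipe obstacles and provides lethal floor and ceiling bounds.
; On BeginPlay, it finds the circular spline tagged "Pipe Path" and spawns the configured number of pipes evenly along it, indexing from 1 to avoid overlap at the loop seam.
; Ceiling and floor collider hits kill the bird, passing the collider's name.
; An older child-actor spawner setup remains unconnected.
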(event `self.ReceiveBeginPlay`
  (`self.Spawn Pipes`))

(event `self.DeathCollider_Ceiling.OnComponentHit`
  (params (HitComponent :type "PrimitiveComponent Object Reference") (OtherActor :type "Actor Object Reference") (OtherComp :type "PrimitiveComponent Object Reference") (NormalImpulse :type "Vector Structure") (Hit :type "HitResult Structure (by ref)"))
  (bind _asflappy_bird_character_bp (cast `/Game/FlappyBird/FlappyBird_Character_BP` OtherActor))
  (`/Game/FlappyBird/FlappyBird_Character_BP.Kill Bird` _asflappy_bird_character_bp "DeathCollider_Ceiling"))

(event `self.DeathCollider_Floor.OnComponentHit`
  (params (HitComponent :type "PrimitiveComponent Object Reference") (OtherActor :type "Actor Object Reference") (OtherComp :type "PrimitiveComponent Object Reference") (NormalImpulse :type "Vector Structure") (Hit :type "HitResult Structure (by ref)"))
  (bind _asflappy_bird_character_bp (cast `/Game/FlappyBird/FlappyBird_Character_BP` OtherActor))
  (`/Game/FlappyBird/FlappyBird_Character_BP.Kill Bird` _asflappy_bird_character_bp "DeathCollider_Floor"))

(fn `Spawn Pipes`
  (locals (`Circular spline that is the main path` :type "/Game/Background_Spinner/CircularSpline_BP Object Reference"))
  (set `self.Total Number of Pipes` (`self.Total number of pipes`))
  (bind _outactors (`GameplayStatics.GetAllActorsWithTag` "Pipe Path"))
  (bind _ascircular_spline_bp (cast `/Game/Background_Spinner/CircularSpline_BP` (`|GetArrayItem` _outactors)))
  (set `local.Circular spline that is the main path` _ascircular_spline_bp)
  (for _index (range 1 (+ (`self.Total Number of Pipes`) 1))
    (`|SpawnActorFromClass` "/Game/Obstacles/Obstacles_BP.Obstacles_BP_C" (`SplineComponent.GetTransformAtDistanceAlongSpline` (`/Game/Background_Spinner/CircularSpline_BP.Circle_Spline` (`local.Circular spline that is the main path`)) (* _index (/ (`SplineComponent.GetSplineLength` (`/Game/Background_Spinner/CircularSpline_BP.Circle_Spline` (`local.Circular spline that is the main path`))) (`KismetMathLibrary.Conv_IntToDouble` (`self.Total Number of Pipes`)))) "World" false) "AlwaysSpawn" "OverrideRootScale" null null)))

(fn `UserConstructionScript`
  (locals (`Circular Spline that is the main path` :type "/Game/Background_Spinner/CircularSpline_BP Object Reference")))