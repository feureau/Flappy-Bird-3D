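; Flappy Bird pipe obstacle that kills the bird when it hits either pipe and scores a point when it enters the gap.
; On BeginPlay it spreads the top and bottom pipes by an offset distance and matches the score box's height extent to that offset.
; A timeline lerps the actor to a random height at start and again one second after an overlap with the score box ends.
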(event `self.ReceiveBeginPlay`
  (bind _score_collider (`self.Score Collider`))
  (bind (_returnvalue_x _returnvalue_y) (`KismetMathLibrary.BreakVector` (`BoxComponent.GetUnscaledBoxExtent` _score_collider)))
  ;[1 1 1] Move Bottom and Top pipes to a random offset
  ;;[1 1 1] Set bottom pipe into position
  (`SceneComponent.K2_AddWorldTransform` (`self.DeathCollider_Bottom`) (`KismetMathLibrary.MakeTransform` (`KismetMathLibrary.MakeVector` 0.0 0.0 (* (`self.Pipe offset distance`) -1.0))) false false)
  ;;[1 1 1] Set top pipe into position
  (`SceneComponent.K2_AddWorldTransform` (`self.DeathCollider_Top`) (`KismetMathLibrary.MakeTransform` (`KismetMathLibrary.MakeVector` 0.0 0.0 (`self.Pipe offset distance`))) false false)
  ;[1 1 1] Make score collider height the same as pipe distance
  (`BoxComponent.SetBoxExtent` _score_collider (`KismetMathLibrary.MakeVector` _returnvalue_x _returnvalue_y (`self.Pipe offset distance`)) false)
  (`self.Randomize obstacle vertical position`))

(event `Randomize obstacle vertical position`
  (bind (_returnvalue_x _returnvalue_y) (`KismetMathLibrary.BreakVector` (`self.K2_GetActorLocation`)))
  ;[1 1 1] Set the vertical position of the obstacle to a random position based on min max
  (set `self.Obstacle Vertical Position (Randomized)` (`KismetMathLibrary.RandomFloatInRange` 300.0 1000.0))
  (bind (_direction _alpha_for_lerp) (`Timeline|Obstacle movement speed` :!via `PlayFromStart`)
    (:`Update`
      (`self.K2_SetActorLocation` (`KismetMathLibrary.VLerp` (`self.K2_GetActorLocation`) (`KismetMathLibrary.MakeVector` _returnvalue_x _returnvalue_y (`self.Obstacle Vertical Position (Randomized)`)) _alpha_for_lerp)))))

(event `self.DeathCollider_Top.OnComponentHit`
  (params (HitComponent :type "PrimitiveComponent Object Reference") (OtherActor :type "Actor Object Reference") (OtherComp :type "PrimitiveComponent Object Reference") (NormalImpulse :type "Vector Structure") (Hit :type "HitResult Structure (by ref)"))
  ;[1 1 1] If bird collides with top or bottom, kill it.
  (bind _asflappy_bird_character_bp (cast `/Game/FlappyBird/FlappyBird_Character_BP` OtherActor))
  (`/Game/FlappyBird/FlappyBird_Character_BP.Kill Bird` _asflappy_bird_character_bp "DeathCollider_Top"))

(event `self.DeathCollider_Bottom.OnComponentHit`
  (params (HitComponent :type "PrimitiveComponent Object Reference") (OtherActor :type "Actor Object Reference") (OtherComp :type "PrimitiveComponent Object Reference") (NormalImpulse :type "Vector Structure") (Hit :type "HitResult Structure (by ref)"))
  ;[1 1 1] If bird collides with top or bottom, kill it.
  (bind _asflappy_bird_character_bp (cast `/Game/FlappyBird/FlappyBird_Character_BP` OtherActor))
  (`/Game/FlappyBird/FlappyBird_Character_BP.Kill Bird` _asflappy_bird_character_bp "DeathCollider_Bottom"))

(event `self.Score Collider.OnComponentBeginOverlap`
  (params (OverlappedComponent :type "PrimitiveComponent Object Reference") (OtherActor :type "Actor Object Reference") (OtherComp :type "PrimitiveComponent Object Reference") (OtherBodyIndex :type Integer) (bFromSweep :type Boolean) (SweepResult :type "HitResult Structure (by ref)"))
  ;[1 1 1] Increment Score
  (cast `/Game/FlappyBird/FlappyBird_Character_BP` OtherActor)
  (`/Game/FlappyBird_GameMode_BP.Increment Score` (cast `/Game/FlappyBird_GameMode_BP` (`GameplayStatics.GetGameMode`) :!pure true)))

(event `self.Score Collider.OnComponentEndOverlap`
  (params (OverlappedComponent :type "PrimitiveComponent Object Reference") (OtherActor :type "Actor Object Reference") (OtherComp :type "PrimitiveComponent Object Reference") (OtherBodyIndex :type Integer))
  ;[1 1 1] Reposition pipes after it goes offscreen
  (`KismetSystemLibrary.Delay` 1.0)
  (`self.Randomize obstacle vertical position`))

(fn `UserConstructionScript`)